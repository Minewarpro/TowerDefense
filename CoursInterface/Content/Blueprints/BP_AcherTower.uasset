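; Archer tower for a tower-defense game that shoots arrows at enemies in range once placed.
; A sphere overlap maintains the target list and runs a looping shot timer, while the spawned archer turns toward the first target.
; Shots play a rate-scaled montage whose notify spawns the arrow.
; Upgrades apply struct-array stats and meshes per level; a "big tower" tier hides the archer and fires big arrows from its own spawn point.
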(event `TheBigTower`
  (`SceneComponent.SetHiddenInGame` (`/Game/Blueprints/BP_Archer.DefaultSceneRoot` (`self.Archer`)) true true)
  (set `self.IsTheBigTower` true))

(event `self.ReceiveTick`
  (params (DeltaSeconds :type "Float (single-precision)"))
  (bind _defaultsceneroot (`/Game/Blueprints/BP_Archer.DefaultSceneRoot` (`self.Archer`)))
  (bind (_returnvalue_roll _returnvalue_pitch _returnvalue_yaw) (`KismetMathLibrary.BreakRotator` (`KismetMathLibrary.FindLookAtRotation` (`SceneComponent.K2_GetComponentLocation` _defaultsceneroot) (`SceneComponent.K2_GetComponentLocation` (`/Game/Ennemies/BP_Enemy.DefaultSceneRoot` (`|GetArrayItem` (`self.Targets`)))))))
  (if (and (> (`KismetArrayLibrary.Array_Length` (`self.Targets`)) 0) (`self.IsPlaced`))
    (`SceneComponent.K2_SetWorldRotation` _defaultsceneroot (`KismetMathLibrary.MakeRotator` 0.0 0.0 (- _returnvalue_yaw 90.0)) false false)))

(event `SpawnArcher`
  (bind (_returnvalue_location _returnvalue_rotation) (`KismetMathLibrary.BreakTransform` (`SceneComponent.K2_GetComponentToWorld` (`self.ArcherSpawn`))))
  (bind _returnvalue (`|SpawnActorFromClass` "/Game/Blueprints/BP_Archer.BP_Archer_C" (`KismetMathLibrary.MakeTransform` _returnvalue_location _returnvalue_rotation (0.75 0.75 0.75)) "Undefined" "OverrideRootScale" null null))
  (set `self.Archer` _returnvalue))

(event `TimerShot`
  (bind _returnvalue (`KismetSystemLibrary.K2_SetTimerDelegate` (delegate `Shot`) (`self.timeBetweenShot`) true))
  (set `self.ShotTimerEvent` _returnvalue)
  (`self.Shot`)
  (set `self.Can Shoot` false))

(event `Shot`
  (if (`self.IsPlaced`)
    (`|PlayMontage` (`/Game/Blueprints/BP_Archer.SK_Archer` (`self.Archer`)) "/Game/Ennemies/Shooting_Arrow_Montage.Shooting_Arrow_Montage" (/ 4.0 (`self.timeBetweenShot`))
      (:`OnNotifyBegin`
        (bind _returnvalue (`|SpawnActorFromClass` "/Game/Blueprints/BP_Arrow.BP_Arrow_C" (`KismetMathLibrary.MakeTransform` (select `bool` (`self.IsTheBigTower`) :`false` (`SceneComponent.GetSocketLocation` (`/Game/Blueprints/BP_Archer.SK_Archer` (`self.Archer`)) "Bow") :`true` (`SceneComponent.K2_GetComponentLocation` (`self.SUPERMEGABALLSPAWN`)))) "Undefined" "OverrideRootScale" null null))
        (`/Engine/EditorBlueprintResources/StandardMacros.IsValid` (`|GetArrayItem` (`self.Targets`))
          (:`Is Valid`
            (`/Game/Blueprints/BP_Arrow.SpawnArrow` _returnvalue (`self.Damages`) (`self.IsTheBigTower`) self)
            (if (== (`KismetArrayLibrary.Array_Length` (`self.Targets`)) 0)
              (`KismetSystemLibrary.K2_ClearAndInvalidateTimerHandle` (`self.ShotTimerEvent`))))
          (:`Is Not Valid`
            (`self.K2_DestroyActor` _returnvalue)))))))

(event `self.Sphere.OnComponentBeginOverlap`
  (params (OverlappedComponent :type "PrimitiveComponent Object Reference") (OtherActor :type "Actor Object Reference") (OtherComp :type "PrimitiveComponent Object Reference") (OtherBodyIndex :type Integer) (bFromSweep :type Boolean) (SweepResult :type "HitResult Structure (by ref)"))
  (bind _asbp_enemy (cast `/Game/Ennemies/BP_Enemy` OtherActor))
  (`KismetArrayLibrary.Array_Add` (`self.Targets`) _asbp_enemy)
  (if (`self.Can Shoot`)
    (`self.TimerShot`)))

(event `self.Sphere.OnComponentEndOverlap`
  (params (OverlappedComponent :type "PrimitiveComponent Object Reference") (OtherActor :type "Actor Object Reference") (OtherComp :type "PrimitiveComponent Object Reference") (OtherBodyIndex :type Integer))
  (bind _targets (`self.Targets`))
  (cast `/Game/Ennemies/BP_Enemy` OtherActor)
  (for (_array_element _array_index) (`self.Targets`)
    (if (== _array_element OtherActor)
      (`KismetArrayLibrary.Array_Remove` _targets _array_index)
      (if (== (`KismetArrayLibrary.Array_Length` _targets) 0)
        (`KismetSystemLibrary.K2_ClearAndInvalidateTimerHandle` (`self.ShotTimerEvent`))
        (set `self.Can Shoot` true)))))

(event `/Game/Blueprints/BPI_Upgrade.Upgrade`
  (bind _level (`self.Level`))
  (if (< _level (`self.MaxLevel`))
    (set `self.Level` (+ _level 1))
    (`self.Set Upgrade`)))

(event `self.ReceiveBeginPlay`
  (bind (_output_damages _output_timebetweenshot _output_staticmesh _output_archerzlocation _output_towerscale _output_prize) (break `/Game/Blueprints/Struct_UpgradeArcherTower` (`|GetArrayItem` (`self.UpgradeStruct`))))
  (`self.Set Upgrade`)
  (set `self.Prize` _output_prize))

(fn `Set Prize To upgrade`
  (bind (_output_damages _output_timebetweenshot _output_staticmesh _output_archerzlocation _output_towerscale _output_prize) (break `/Game/Blueprints/Struct_UpgradeArcherTower` (`|GetArrayItem` (`self.UpgradeStruct`) (`self.Level`))))
  (if (< (`self.Level`) (`self.MaxLevel`))
    (set `self.PrizeToUpgrade` _output_prize)))

(fn `Set Upgrade`
  (bind _tower (`self.Tower`))
  (bind _archer (`self.Archer`))
  (bind _rootcomponent (`Actor.RootComponent` _archer))
  (bind (_returnvalue_x _returnvalue_y) (`KismetMathLibrary.BreakVector` (`SceneComponent.K2_GetComponentLocation` _rootcomponent)))
  (bind (_output_damages _output_timebetweenshot _output_staticmesh _output_archerzlocation _output_towerscale) (break `/Game/Blueprints/Struct_UpgradeArcherTower` (`|GetArrayItem` (`self.UpgradeStruct`) (- (`self.Level`) 1))))
  (bind (_output_damages_2 _output_timebetweenshot_2 _output_staticmesh_2 _output_archerzlocation_2 _output_towerscale_2 _output_prize _output_is_thebigtower) (break `/Game/Blueprints/Struct_UpgradeArcherTower` (`|GetArrayItem` (`self.UpgradeStruct`) (- (`self.Level`) 1))))
  (`|ExecutionSequence`
    (:`then_0`
      (`self.Set Prize To upgrade`)
      (set `self.Damages` _output_damages)
      (set `self.timeBetweenShot` _output_timebetweenshot)
      (`StaticMeshComponent.SetStaticMesh` _tower _output_staticmesh)
      (for _index (range 100000)
        (bind _returnvalue (`StaticMesh.GetMaterial` _output_staticmesh _index))
        (`/Engine/EditorBlueprintResources/StandardMacros.IsValid` _returnvalue
          (:`Is Valid`
            (`PrimitiveComponent.SetMaterial` _tower _index _returnvalue))
          (:`Is Not Valid`
            (break))))
      (`SceneComponent.K2_SetRelativeTransform` _tower (`KismetMathLibrary.MakeTransform` (0.0 0.0 0.0) (struct :`Yaw` 90.0) _output_towerscale) false false)
      (`SceneComponent.K2_SetRelativeLocation` (`self.ArcherSpawn`) (`KismetMathLibrary.MakeVector` 0.0 0.0 _output_archerzlocation) false false)
      (`/Engine/EditorBlueprintResources/StandardMacros.IsValid` _archer
        (:`Is Valid`
          (`SceneComponent.K2_SetWorldLocation` _rootcomponent (`KismetMathLibrary.MakeVector` _returnvalue_x _returnvalue_y _output_archerzlocation) false false)
          (`|ExecutionSequence`
            (:`then_0`
              (if (== (`self.Level`) (`self.MaxLevel`))
                (set `self.CanUpgrade` false)))
            (:`then_1`
              (if _output_is_thebigtower
                (`self.TheBigTower`)))))))
    (:`then_1`
      (if (not (`self.Can Shoot`))
        (`KismetSystemLibrary.K2_ClearAndInvalidateTimerHandle` (`self.ShotTimerEvent`))
        (`self.TimerShot`)))
    (:`then_2`
      (set `self.Damage` (`self.Damages`))
      (set `self.TimeBetweenShots` (`self.timeBetweenShot`)))))

(fn `SetTargetForArrows`
  (returns (DefaultSceneRoot :type "SceneComponent Object Reference"))
  (return (`/Game/Ennemies/BP_Enemy.DefaultSceneRoot` (`|GetArrayItem` (`self.Targets`)))))

(fn `UserConstructionScript`
  (`parent.UserConstructionScript`)
  (set `self.MaxLevel` (`KismetArrayLibrary.Array_Length` (`self.UpgradeStruct`))))