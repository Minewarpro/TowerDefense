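; Guard tower Blueprint that spawns three BP_Gard units and upgrades them alongside itself.
; SpawnGard places the guards at a given transform, spread side by side along their local X axis.
; SetUpgrade reads the current level's UpgradeStruct entry for stats, mesh, scale and next upgrade price, and mirrors damage and attack timing into parent variables.
; Upgrade raises the level up to MaxLevel and pushes damage, max life and attack interval to the guards.
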(event `SpawnGard`
  (params (SpawnTransform :type "Transform Structure"))
  (set `self.Spawn Transform Location` SpawnTransform_Location)
  (set `self.Spawn Transform Rotation` SpawnTransform_Rotation)
  (`|ExecutionSequence`
    (:`then_0`
      (bind _returnvalue (`|SpawnActorFromClass` "/Game/Blueprints/BP_Gard.BP_Gard_C" (`KismetMathLibrary.MakeTransform` (`self.Spawn Transform Location`) (`self.Spawn Transform Rotation`) (0.75 0.75 0.75)) "Undefined" "OverrideRootScale" null null))
      (bind _output_get (set `self.Gard_1` _returnvalue))
      (bind _rootcomponent (`Actor.RootComponent` _output_get))
      (bind (_returnvalue_location _returnvalue_rotation _returnvalue_scale) (`KismetMathLibrary.BreakTransform` (`SceneComponent.K2_GetComponentToWorld` (`Actor.RootComponent` _output_get))))
      (`SceneComponent.K2_SetWorldTransform` _rootcomponent (`KismetMathLibrary.MakeTransform` (`self.Spawn Transform Location`) (`self.Spawn Transform Rotation`) _returnvalue_scale) false false)
      (`SceneComponent.K2_AddLocalOffset` _rootcomponent (-150.0 0.0 0.0) false false))
    (:`then_1`
      (bind _returnvalue_2 (`|SpawnActorFromClass` "/Game/Blueprints/BP_Gard.BP_Gard_C" (`KismetMathLibrary.MakeTransform` (`self.Spawn Transform Location`) (`self.Spawn Transform Rotation`) (0.75 0.75 0.75)) "Undefined" "OverrideRootScale" null null))
      (bind _output_get_2 (set `self.Gard_3` _returnvalue_2))
      (bind _rootcomponent_2 (`Actor.RootComponent` _output_get_2))
      (bind (_returnvalue_location_2 _returnvalue_rotation_2 _returnvalue_scale_2) (`KismetMathLibrary.BreakTransform` (`SceneComponent.K2_GetComponentToWorld` (`Actor.RootComponent` _output_get_2))))
      (`SceneComponent.K2_SetWorldTransform` _rootcomponent_2 (`KismetMathLibrary.MakeTransform` (`self.Spawn Transform Location`) (`self.Spawn Transform Rotation`) _returnvalue_scale_2) false false)
      (`SceneComponent.K2_AddLocalOffset` _rootcomponent_2 (150.0 0.0 0.0) false false))
    (:`then_2`
      (bind _returnvalue_3 (`|SpawnActorFromClass` "/Game/Blueprints/BP_Gard.BP_Gard_C" (`KismetMathLibrary.MakeTransform` (`self.Spawn Transform Location`) (`self.Spawn Transform Rotation`) (0.75 0.75 0.75)) "Undefined" "OverrideRootScale" null null))
      (bind _output_get_3 (set `self.Gard_2` _returnvalue_3))
      (bind (_returnvalue_location_3 _returnvalue_rotation_3 _returnvalue_scale_3) (`KismetMathLibrary.BreakTransform` (`SceneComponent.K2_GetComponentToWorld` (`Actor.RootComponent` _output_get_3))))
      (`SceneComponent.K2_SetWorldTransform` (`Actor.RootComponent` _output_get_3) (`KismetMathLibrary.MakeTransform` (`self.Spawn Transform Location`) (`self.Spawn Transform Rotation`) _returnvalue_scale_3) false false))))

(event `/Game/Blueprints/BPI_Upgrade.Upgrade`
  (bind _level (`self.Level`))
  (if (< _level (`self.MaxLevel`))
    (set `self.Level` (+ _level 1))
    (`self.Set Upgrade`)
    (`/Game/Blueprints/BP_Gard.Upgrade` (`self.Gard_1`) (`self.Damages`) (`self.MaxLife`) (`self.timeBetweenAttacks`) 0.0)
    (`/Game/Blueprints/BP_Gard.Upgrade` (`self.Gard_2`) (`self.Damages`) (`self.MaxLife`) (`self.timeBetweenAttacks`) 0.0)
    (`/Game/Blueprints/BP_Gard.Upgrade` (`self.Gard_3`) (`self.Damages`) (`self.MaxLife`) (`self.timeBetweenAttacks`) 0.0)))

(event `self.ReceiveBeginPlay`
  (bind (_output_damages _output_maxlife _output_timebetweenattacks _output_staticmesh _output_towerscale _output_prize) (break `/Game/Blueprints/Struct_UpgradeGardTower` (`|GetArrayItem` (`self.UpgradeStruct`))))
  (`self.Set Upgrade`)
  (set `self.Prize` _output_prize))

(fn `Set Prize To Upgrade`
  (bind (_output_damages _output_maxlife _output_timebetweenattacks _output_staticmesh _output_towerscale _output_prize) (break `/Game/Blueprints/Struct_UpgradeGardTower` (`|GetArrayItem` (`self.UpgradeStruct`) (`self.Level`))))
  (if (< (`self.Level`) (`self.MaxLevel`))
    (set `self.PrizeToUpgrade` _output_prize)))

(fn `Set Upgrade`
  (bind _tower (`self.Tower`))
  (bind (_output_damages _output_maxlife _output_timebetweenattacks _output_staticmesh _output_towerscale _output_prize _output_voldevie) (break `/Game/Blueprints/Struct_UpgradeGardTower` (`|GetArrayItem` (`self.UpgradeStruct`) (- (`self.Level`) 1))))
  (`|ExecutionSequence`
    (:`then_0`
      ;[0.08333 0.08333 0.08333] Set Visuel
      (`self.Set Prize To Upgrade`)
      (set `self.Damages` _output_damages)
      (set `self.MaxLife` _output_maxlife)
      (set `self.timeBetweenAttacks` _output_timebetweenattacks)
      (set `self.VolDeVie` _output_voldevie)
      (`StaticMeshComponent.SetStaticMesh` _tower _output_staticmesh)
      (`SceneComponent.K2_SetRelativeTransform` _tower (`KismetMathLibrary.MakeTransform` (0.0 0.0 0.0) (struct :`Yaw` 90.0) _output_towerscale) false false)
      ;[0.07292 0.07292 0.07292] Detect the last Upgrade
      (if (== (`self.Level`) (`self.MaxLevel`))
        (set `self.CanUpgrade` false)))
    (:`then_1`
      ;[0.08854 0.08854 0.08854] Set Parent Variables
      (set `self.Damage` (`self.Damages`))
      (set `self.TimeBetweenShots` (`self.timeBetweenAttacks`)))))

(fn `UserConstructionScript`
  (`parent.UserConstructionScript`))