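; BP_SplinePath is an enemy wave spawner that sends enemies along its spline.
; StartWave runs a looping timer that spawns batches at the spline and calls MoveObject on each, stopping at the wave's quota.
; Per-wave arrays, resized to MaxWaves in construction, set base type, counts and spawn-position type exceptions.
; OnEnemyDie counts deaths and re-enables the start button once the wave's total is reached.
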(event `OnEnemyDie`
  (set `self.CurrentEnmenyDead` (+ (`self.CurrentEnmenyDead`) 1))
  (`self.EndWaveCheck`))

(event `StartWave`
  (params (StartWaveButton :type "Button Object Reference"))
  (set `self.Start Wave Button` StartWaveButton)
  (set `self.CurrentEnmenyDead` 0)
  (set `self.CurrentWave` (+ (`self.CurrentWave`) 1))
  (bind _returnvalue (`KismetSystemLibrary.K2_SetTimerDelegate` (delegate `Spawn Troll`) (`self.EnemySpawnRate`) true))
  (set `self.StartWaveEvent` _returnvalue))

(event `Spawn Troll`
  (set `self.ActorToSpawn` (`|GetArrayItem` (`self.BaseEnemyType`) (- (`self.CurrentWave`) 1)))
  (for _ (range (`|GetArrayItem` (`self.NumberOfEnnemySpawnAtSameTime`) (- (`self.CurrentWave`) 1)))
    (`self.TypeEnemyToSpawn`)
    (set `self.NumberEnemySpawned` (+ (`self.NumberEnemySpawned`) 1))
    (bind _returnvalue (`|SpawnActorFromClass` (`self.ActorToSpawn`) (`KismetMathLibrary.MakeTransform` (`SceneComponent.K2_GetComponentLocation` (`self.Spline`))) "Undefined" "OverrideRootScale" null null))
    (`/Game/Ennemies/BP_Enemy.MoveObject` _returnvalue self _returnvalue)
    (`self.NumberEnemySpawnedCheck`)))

(fn `EndWaveCheck`
  (if (== (`self.CurrentEnmenyDead`) (`|GetArrayItem` (`self.NumberEnemyPerWave`) (- (`self.CurrentWave`) 1)))
    (set `Widget.bIsEnabled` true (`self.Start Wave Button`))))

(fn `NumberEnemySpawnedCheck`
  (if (== (`|GetArrayItem` (`self.NumberEnemyPerWave`) (- (`self.CurrentWave`) 1)) (`self.NumberEnemySpawned`))
    (`KismetSystemLibrary.K2_ClearAndInvalidateTimerHandle` (`self.StartWaveEvent`))
    (set `self.NumberEnemySpawned` 0)))

(fn `TypeEnemyToSpawn`
  (for (_array_element _array_index) (`self.Exeptions`)
    (if (== _array_index (- (`self.CurrentWave`) 1))
      (for _array_element_2 (break `/Game/Ennemies/Struct_Exeptions` _array_element)
        (if (== (- (`.SpawnPosition_6_E9B8FEED4FF2972B8DFB7F9F37022CB4` (break `/Game/Ennemies/Struct_Exeption` _array_element_2)) 1) (`self.NumberEnemySpawned`))
          (set `self.ActorToSpawn` (break `/Game/Ennemies/Struct_Exeption` _array_element_2)))))))

(fn `UserConstructionScript`
  (bind _maxwaves (`self.MaxWaves`))
  (`KismetArrayLibrary.Array_Resize` (`self.Exeptions`) _maxwaves)
  (`KismetArrayLibrary.Array_Resize` (`self.NumberEnemyPerWave`) _maxwaves)
  (`KismetArrayLibrary.Array_Resize` (`self.NumberOfEnnemySpawnAtSameTime`) _maxwaves)
  (`KismetArrayLibrary.Array_Resize` (`self.BaseEnemyType`) _maxwaves))