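; BP_Gard is an upgradeable guard that automatically fights BP_Enemy actors entering its sphere, with a WG_Gard life bar.
; Overlaps maintain an enemy array, call StartCombat on each newcomer and drive a looping attack timer.
; Attack montage speed scales with attack interval, and its notify hits the first enemy and applies lifesteal (VolDeVie).
; Death hides the actor and clears targets rather than destroying it, so Respawn can restore it.
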(event `Upgrade`
  (params (Damage :type "Float (double-precision)") (MaxLife :type "Float (double-precision)") (TimeBetweenAttacks :type "Float (single-precision)") (PercentVolDeVie :type "Float (double-precision)"))
  ;[0.08854 0.08854 0.08854] Upgrade Set Variables
  (set `self.Damage` Damage)
  (set `self.MaxLife` MaxLife)
  (set `self.TimeBetweenAttacks` TimeBetweenAttacks)
  (set `self.CurrentLife` (`self.MaxLife`))
  (set `self.PercentVolDeVie` PercentVolDeVie))

(event `self.ReceiveBeginPlay`
  ;[0.06771 0.06771 0.06771] Begin Play
  (`self.InitializationVariables`)
  (bind _aswg_gard (cast `/Game/UI/WG_Gard` (`WidgetComponent.GetUserWidgetObject` (`self.LifeBar`))))
  (set `/Game/UI/WG_Gard.ControllerRef` self _aswg_gard))

(event `TakeDamage`
  (params (Damages :type "Float (double-precision)"))
  ;[0.07292 0.07292 0.07292] Take Damage
  (bind _output_get (set `self.CurrentLife` (- (`self.CurrentLife`) Damages)))
  (if (<= _output_get 0.0)
    (`self.Die`)))

(event `Attack`
  (bind _output (`|GetArrayItem` (`self.EnemyArray`)))
  ;[0.07812 0.07812 0.07812] Attack
  (if (not (`self.IsDead`))
    ;;[0.4331 0.8069 1] Animation
    (`|PlayMontage` (`self.Gard`) "/Game/Ennemies/Attack_Montage.Attack_Montage" (/ 2.0 (`self.TimeBetweenAttacks`))
      (:`OnNotifyBegin`
        ;;[0.6614 1 0.655] Send Info Get Hit To Target
        (`/Engine/EditorBlueprintResources/StandardMacros.IsValid` _output
          (:`Is Valid`
            (`/Game/Ennemies/BP_Enemy.GetHit` _output (`self.Damage`))
            (`self.VolDeVie`))
          (:`Is Not Valid`
            _))
        ;;[1 0.5365 0.5819] Stop Attack
        (if (== (`KismetArrayLibrary.Array_Length` (`self.EnemyArray`)) 0)
          (`KismetSystemLibrary.K2_ClearAndInvalidateTimerHandle` (`self.AttackTimerEvent`)))))))

(event `self.Sphere.OnComponentBeginOverlap`
  (params (OverlappedComponent :type "PrimitiveComponent Object Reference") (OtherActor :type "Actor Object Reference") (OtherComp :type "PrimitiveComponent Object Reference") (OtherBodyIndex :type Integer) (bFromSweep :type Boolean) (SweepResult :type "HitResult Structure (by ref)"))
  ;[0.0625 0.0625 0.0625] Add and Remove Enemy of Array
  (if (not (`self.IsDead`))
    (bind _asbp_enemy (cast `/Game/Ennemies/BP_Enemy` OtherActor))
    (`KismetArrayLibrary.Array_Add` (`self.EnemyArray`) _asbp_enemy)
    (`/Game/Ennemies/BP_Enemy.StartCombat` _asbp_enemy self)
    (if (`self.CanAttack`)
      (bind _returnvalue (`KismetSystemLibrary.K2_SetTimerDelegate` (delegate `Attack`) (`self.TimeBetweenAttacks`) true))
      (set `self.AttackTimerEvent` _returnvalue)
      (`self.Attack`)
      (set `self.CanAttack` false))))

(event `self.Sphere.OnComponentEndOverlap`
  (params (OverlappedComponent :type "PrimitiveComponent Object Reference") (OtherActor :type "Actor Object Reference") (OtherComp :type "PrimitiveComponent Object Reference") (OtherBodyIndex :type Integer))
  (bind _enemyarray (`self.EnemyArray`))
  ;[0.0625 0.0625 0.0625] Add and Remove Enemy of Array
  (if (not (`self.IsDead`))
    (cast `/Game/Ennemies/BP_Enemy` OtherActor)
    (for (_array_element _array_index) (`self.EnemyArray`)
      (if (== _array_element OtherActor)
        (`KismetArrayLibrary.Array_Remove` _enemyarray _array_index)
        (if (== (`KismetArrayLibrary.Array_Length` _enemyarray) 0)
          (`KismetSystemLibrary.K2_ClearAndInvalidateTimerHandle` (`self.AttackTimerEvent`))
          (set `self.CanAttack` true))))))

(fn `Die`
  (set `self.IsDead` true)
  (`self.SetActorHiddenInGame` true)
  (`KismetArrayLibrary.Array_Clear` (`self.EnemyArray`)))

(fn `InitializationVariables`
  (set `self.CurrentLife` (`self.MaxLife`)))

(fn `Respawn`
  (set `self.IsDead` false)
  (`self.SetActorHiddenInGame` false)
  (set `self.CurrentLife` (`self.MaxLife`))
  (set `self.CanAttack` true))

(fn `UserConstructionScript`)

(fn `VolDeVie`
  (bind _percentvoldevie (`self.PercentVolDeVie`))
  (bind _returnvalue (+ (`self.CurrentLife`) (* (`self.Damage`) (/ _percentvoldevie 100.0))))
  (if (!= _percentvoldevie 0.0)
    (if (> _returnvalue (`self.MaxLife`))
      (set `self.CurrentLife` (`self.MaxLife`))
      (else
        (set `self.CurrentLife` _returnvalue)))))