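; BP_TutoManager runs the tutorial by flagging the player controller and showing the tutorial UI.
; On BeginPlay it finds the BP_CustomPlayerController, sets its Tuto flag, then creates a WG_Tuto widget with references to that controller and itself and adds it to the viewport.
; Its NextPanel function increments a PanelNumber counter to track the current panel.
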(event `self.ReceiveBeginPlay`
  ;[0.125 0.125 0.125] Create Tutorial UI
  (`|ExecutionSequence`
    (:`then_0`
      (bind _returnvalue (`GameplayStatics.GetActorOfClass` "/Game/ThirdPerson/Blueprints/BP_CustomPlayerController.BP_CustomPlayerController_C"))
      (bind _output_get (set `self.PlayerControllerRef` _returnvalue))
      (set `/Game/ThirdPerson/Blueprints/BP_CustomPlayerController.Tuto` true _output_get))
    (:`then_1`
      (bind _returnvalue_2 (`|CreateWidget` "/Game/UI/WG_Tuto.WG_Tuto_C" null (`self.PlayerControllerRef`) self))
      (`UserWidget.AddToViewport` _returnvalue_2 0))))

(fn `NextPanel`
  (set `self.PanelNumber` (+ (`self.PanelNumber`) 1)))

(fn `UserConstructionScript`)