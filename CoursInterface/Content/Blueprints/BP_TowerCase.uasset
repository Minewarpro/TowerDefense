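; BP_TowerCase is a tower build slot that takes a placed tower and closes itself.
; AddTower stores the tower and casts it, spawning a guard at the GardSpawn transform for a guard tower or calling SpawnArcher for an archer tower.
; It then hides the sign and rect light and clears Open.
; The construction script positions and rotates the guard spawn point and its Scene component from exposed distance and rotation variables.
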(event `AddTower`
  (params (CurrentTower :type "/Game/Blueprints/BP_Tower Object Reference"))
  ;[1 1 1] Pas très jolie je sais / Je peux généraliser
  (bind _output_get (set `self.Current Tower` CurrentTower))
  (bind _asbp_gard_tower (cast `/Game/Blueprints/BP_GardTower` _output_get)
    (:`then`
      (`/Game/Blueprints/BP_GardTower.SpawnGard` _asbp_gard_tower (`SceneComponent.K2_GetComponentToWorld` (`self.GardSpawn`))))
    (:`CastFailed`
      (bind _asbp_acher_tower (cast `/Game/Blueprints/BP_AcherTower` CurrentTower)
        (:`then`
          (`/Game/Blueprints/BP_AcherTower.SpawnArcher` _asbp_acher_tower))
        (:`CastFailed`
          _))))
  (`SceneComponent.SetHiddenInGame` (`self.signs_sign1`) true false)
  (`SceneComponent.SetHiddenInGame` (`self.RectLight`) true false)
  (set `self.Open` false))

(fn `UserConstructionScript`
  (bind _gardspawn (`self.GardSpawn`))
  (`SceneComponent.K2_SetRelativeLocation` _gardspawn (`KismetMathLibrary.MakeVector` 0.0 (`self.GradSpawnDistance`)) false false)
  (`SceneComponent.K2_SetWorldRotation` _gardspawn (`KismetMathLibrary.MakeRotator` 0.0 0.0 (`self.GardRotation`)) false false)
  (`SceneComponent.K2_SetWorldRotation` (`self.Scene`) (`KismetMathLibrary.MakeRotator` 0.0 0.0 (`self.GardSpawnRotation`)) false false))