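; BP_Arrow is a tower-fired homing projectile that damages the first BP_Enemy it overlaps, then destroys itself.
; SpawnArrow stores tower and damage, asks the tower for a target component, and feeds it to ProjectileMovement homing.
; The big-arrow variant, the last upgrade's death ball, shows its Core, suspends gravity and scales Sphere via a timeline.
; It then restores gravity and re-queries the target, self-destructing if none is valid.
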(event `ModifyVariables`
  (params (Damages :type "Float (double-precision)"))
  (set `self.Damages` Damages))

(event `SpawnArrow`
  (params (Damages :type "Float (double-precision)") (Is_TheBigArrow :type Boolean) (Tower :type "/Game/Blueprints/BP_AcherTower Object Reference"))
  (bind _sphere (`self.Sphere`))
  (bind (_returnvalue_location _returnvalue_rotation) (`KismetMathLibrary.BreakTransform` (`SceneComponent.GetRelativeTransform` _sphere)))
  ;[0.06771 0.06771 0.06771] On Arrow Spawn
  ;;[0.4643 0.7628 1] Set Target And Variables
  (bind _output_get (set `self.Tower` Tower))
  (bind _defaultsceneroot (`self.GetTarget` _output_get))
  (set `self.Default Scene Root` _defaultsceneroot)
  (`self.ModifyVariables` Damages)
  (if Is_TheBigArrow
    ;;[1 0.2135 0.2135] Visuel Pour la Boule de la mort ( boule rouge derniere upgrade )
    (`SceneComponent.SetHiddenInGame` (`self.Core`) false true)
    (`SceneComponent.SetHiddenInGame` (`self.Sphere`) true false)
    (set `ProjectileMovementComponent.ProjectileGravityScale` 0.0 (`self.ProjectileMovement`))
    (bind (_direction _scale) (`Timeline|Scale Timeline` :!via `PlayFromStart`)
      (:`Update`
        (bind _returnvalue (* _scale 0.8))
        (`SceneComponent.K2_SetRelativeTransform` _sphere (`KismetMathLibrary.MakeTransform` _returnvalue_location _returnvalue_rotation (`KismetMathLibrary.MakeVector` _returnvalue _returnvalue _returnvalue)) false false))
      (:`Finished`
        (set `ProjectileMovementComponent.ProjectileGravityScale` 1.0 (`self.ProjectileMovement`))
        (bind _defaultsceneroot_2 (`self.GetTarget` (`self.Tower`)))
        (bind _output_get_2 (set `self.Default Scene Root` _defaultsceneroot_2))
        (`/Engine/EditorBlueprintResources/StandardMacros.IsValid` _output_get_2
          (:`Is Valid`
            (set `ProjectileMovementComponent.HomingTargetComponent` (`self.Default Scene Root`) (`self.ProjectileMovement`)))
          (:`Is Not Valid`
            (`self.K2_DestroyActor`)))))
    (else
      ;;[1 1 1] Set Homing Pour la direction de l'arrow
      (set `ProjectileMovementComponent.HomingTargetComponent` (`self.Default Scene Root`) (`self.ProjectileMovement`)))))

(event `self.Sphere.OnComponentBeginOverlap`
  (params (OverlappedComponent :type "PrimitiveComponent Object Reference") (OtherActor :type "Actor Object Reference") (OtherComp :type "PrimitiveComponent Object Reference") (OtherBodyIndex :type Integer) (bFromSweep :type Boolean) (SweepResult :type "HitResult Structure (by ref)"))
  ;[0.06771 0.06771 0.06771] When Touch Enemy
  (bind _asbp_enemy (cast `/Game/Ennemies/BP_Enemy` OtherActor))
  (`self.K2_DestroyActor`)
  (`/Game/Ennemies/BP_Enemy.GetHit` _asbp_enemy (`self.Damages`)))

(fn `GetTarget`
  (params (Tower :type "/Game/Blueprints/BP_AcherTower Object Reference"))
  (returns (DefaultSceneRoot :type "SceneComponent Object Reference"))
  (bind _defaultsceneroot (`/Game/Blueprints/BP_AcherTower.SetTargetForArrows` Tower))
  (return _defaultsceneroot))

(fn `UserConstructionScript`
  (`SceneComponent.SetHiddenInGame` (`self.Core`) true true))