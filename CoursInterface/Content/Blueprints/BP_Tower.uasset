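; BP_Tower is a tower Blueprint that gives visual feedback for selection and for an on/off "case" state.
; Selected and UnSelected toggle custom depth rendering on the Tower component.
; The construction script caches the component's original material as RealMaterial, then applies M_TowerError as the initial look.
; OnCase restores the cached material and OffCase switches back to the error material.
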(event `UnSelected`
  (`PrimitiveComponent.SetRenderCustomDepth` (`self.Tower`) false))

(event `Selected`
  (`PrimitiveComponent.SetRenderCustomDepth` (`self.Tower`) true))

(event `OnCase`
  (`PrimitiveComponent.SetMaterial` (`self.Tower`) 0 (`self.RealMaterial`)))

(event `OffCase`
  (`PrimitiveComponent.SetMaterial` (`self.Tower`) 0 "/Game/Materials/M_TowerError.M_TowerError"))

(fn `UserConstructionScript`
  (bind _tower (`self.Tower`))
  (set `self.RealMaterial` (`PrimitiveComponent.GetMaterial` _tower 0))
  (`PrimitiveComponent.SetMaterial` _tower 0 "/Game/Materials/M_TowerError.M_TowerError"))