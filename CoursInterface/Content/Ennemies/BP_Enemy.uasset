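; Tower defense style enemy that walks a spline path, fights guards on the way and damages the player controller when it reaches the end.
; A timeline sized by TimeToComplete moves it along the spline with a random X offset.
; Combat pauses the timeline and loops a timed montage attack, damaging the guard on notify and resuming movement once it dies.
; Death notifies the spline path and gives gold, including at path end.
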(event `Attack`
  (bind _gard (`self.Gard`))
  (`|PlayMontage` (`self.SkeletalMesh`) "/Game/Ennemies/Attack_Montage.Attack_Montage"
    (:`OnNotifyBegin`
      (`/Game/Blueprints/BP_Gard.TakeDamage` _gard (`self.DamagesToGard`))
      (if (`/Game/Blueprints/BP_Gard.IsDead` _gard)
        (`self.EndCombat`)))))

(event `StartCombat`
  (params (Gard :type "/Game/Blueprints/BP_Gard Object Reference"))
  (set `self.Gard` Gard)
  (set `self.IsMoving` false)
  (`TimelineComponent.Stop` (`self.Move Object TImeline`))
  (bind _returnvalue (`KismetSystemLibrary.K2_SetTimerDelegate` (delegate `Attack`) 2.0 true))
  (set `self.AttackTimerEvent` _returnvalue)
  (`self.Attack`))

(event `EndCombat`
  (bind _target (`self.Target`))
  (set `self.IsMoving` true)
  (`TimelineComponent.Play` (`self.Move Object TImeline`))
  (`KismetSystemLibrary.K2_ClearAndInvalidateTimerHandle` (`self.AttackTimerEvent`))
  (`/Engine/EditorBlueprintResources/StandardMacros.IsValid` _target
    (:`Is Valid`
      (`Character.StopAnimMontage` _target "/Game/Ennemies/Attack_Montage.Attack_Montage"))))

(event `self.ReceiveBeginPlay`
  (bind _returnvalue (`GameplayStatics.GetActorOfClass` "/Game/Blueprints/BP_SplinePath.BP_SplinePath_C"))
  (set `self.SplineRef` _returnvalue)
  (bind _returnvalue_2 (`GameplayStatics.GetActorOfClass` "/Game/ThirdPerson/Blueprints/BP_CustomPlayerController.BP_CustomPlayerController_C"))
  (set `self.PlayerControllerRef` _returnvalue_2))

(event `GetHit`
  (params (Damage :type "Float (double-precision)"))
  (bind _output_get (set `self.CurrentLife` (- (`self.CurrentLife`) Damage)))
  (if (<= _output_get 0.0)
    (`self.KillEnemy`)))

(event `EndCourse`
  (`/Game/ThirdPerson/Blueprints/BP_CustomPlayerController.TakeDamage` (`self.PlayerControllerRef`) (`self.Damages`))
  (`self.KillEnemy`))

(event `MoveObject`
  (params (`Spline to follow` :type "/Game/Blueprints/BP_SplinePath Object Reference") (TargetRef :type "/Game/Ennemies/BP_Enemy Object Reference"))
  (bind _spline (`/Game/Blueprints/BP_SplinePath.Spline` (`self.SplineLineToFollow`)))
  (`|ExecutionSequence`
    (:`then_0`
      (set `self.RandomWay` (`KismetMathLibrary.RandomFloatInRange` -100.0 100.0))
      (set `self.SplineLineToFollow` `Spline to follow`)
      (set `self.IsMoving` true)
      (`TimelineComponent.SetPlayRate` (`self.Move Object TImeline`) (/ 1.0 (`self.TimeToComplete`)))
      (bind (_direction _moving) (`Timeline|Move Object TImeline`)
        (:`Update`
          (bind _returnvalue (`KismetMathLibrary.Lerp` 0.0 (`SplineComponent.GetSplineLength` (`/Game/Blueprints/BP_SplinePath.Spline` (`self.SplineLineToFollow`))) _moving))
          (bind (_returnvalue_x _returnvalue_y _returnvalue_z) (`KismetMathLibrary.BreakVector` (`SplineComponent.GetLocationAtDistanceAlongSpline` _spline _returnvalue "World")))
          (`self.K2_SetActorTransform` (`KismetMathLibrary.MakeTransform` (`KismetMathLibrary.MakeVector` (+ _returnvalue_x (`self.RandomWay`)) _returnvalue_y _returnvalue_z) (`SplineComponent.GetRotationAtDistanceAlongSpline` _spline _returnvalue "Local"))))
        (:`Finished`
          (`self.EndCourse`))))
    (:`then_1`
      (message `/Game/Ennemies/BPI_SpawnEnemy.Spawn Enemy` TargetRef)
      (set `self.CurrentLife` (`self.MaxLife`))
      (bind _aswg_enemy (cast `/Game/UI/WG_Enemy` (`WidgetComponent.GetUserWidgetObject` (`self.Widget`))))
      (bind _output_get (set `self.As WG Enemy` _aswg_enemy))
      (set `/Game/UI/WG_Enemy.ControllerRef` self _output_get))))

(fn `KillEnemy`
  (`self.K2_DestroyActor`)
  (`/Game/Blueprints/BP_SplinePath.OnEnemyDie` (`self.SplineRef`))
  (`/Game/ThirdPerson/Blueprints/BP_CustomPlayerController.GetGold` (`self.PlayerControllerRef`) (`self.Gold`)))

(fn `UserConstructionScript`)