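; Enemy Blueprint, named as the foe to avoid, that supplies its own stats for combat, course timing and gold.
; When the SpawnEnemy event fires, InitializeVariables copies its damage, damage to guards, course completion time, maximum health and gold values into the working stat variables.
; The construction script only calls the parent's, and the file holds no other behavior.
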(event `/Game/Ennemies/BPI_SpawnEnemy.Spawn Enemy`
  (`self.InitializeVariables`))

(fn `InitializeVariables`
  (set `self.Damages` (`self.Damage`))
  (set `self.TimeToComplete` (`self.TimeToCompleteCourse`))
  (set `self.MaxLife` (`self.HealthMax`))
  (set `self.DamagesToGard` (`self.DamagesToGards`))
  (set `self.Gold` (`self.Golds`)))

(fn `UserConstructionScript`
  (`parent.UserConstructionScript`))